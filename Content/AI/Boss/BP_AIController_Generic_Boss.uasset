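; Generic boss AI controller that runs the boss behavior tree and manages an on-screen boss health bar.
; BeginPlay starts BT_AI_Boss.
; Combat activation creates the health bar widget and adds it to the viewport, and deactivation removes and clears it.
; While the widget exists, Tick sets its fill from current health divided by max health.
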(event `self.ReceiveBeginPlay`
  (`self.RunBehaviorTree` "/Game/AI/Boss/BT_AI_Boss.BT_AI_Boss"))

(event `ActivateBossCombat`
  (bind _returnvalue (`|CreateWidget` "/Game/UI/BossHealthBar.BossHealthBar_C"))
  (bind _output_get (set `self.Boss Health bar` _returnvalue))
  (`UserWidget.AddToViewport` _output_get 0))

(event `Deactivate Boss Combat`
  (`Widget.RemoveFromParent` (`self.Boss Health bar`))
  (set `self.Boss Health bar` null))

(event `self.ReceiveTick`
  (params (DeltaSeconds :type "Float (single-precision)"))
  (bind _boss_health_bar (`self.Boss Health bar`)
    (:`then`
      (`ProgressBar.SetPercent` (`/Game/UI/BossHealthBar.HealthBar` _boss_health_bar) (/ (`self.Health`) (`self.MaxHealtrh`))))
    (:`else`)))

(fn `UserConstructionScript`
  (`parent.UserConstructionScript`))