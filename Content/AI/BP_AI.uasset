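; Enemy AI character for melee combat that the player can fight or assassinate from behind.
; A behavior-tree-facing Attack function drives an indexed montage combo with saved inputs, while timer-looped sword traces and a single sphere trace damage "Damageable" actors.
; Incoming damage interrupts combos, plays random hit reactions with knockback, and ragdolls when BPCPlayerStats.DecreaseHealth returns true.
; An overlap radius shows the camera-facing assassination prompt; StealthbBackAssassin plays the victim montage, triggers delayed ragdoll and returns alignment transforms.
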(event `self.ReceiveBeginPlay`
  (bind _asdummy_healthbar (cast `/Game/UI/DummyHealthbar` (`WidgetComponent.GetWidget` (`self.HealthBar `))))
  (set `self.Healthbar UI` _asdummy_healthbar))

(event `self.ReceiveTick`
  (params (DeltaSeconds :type "Float (single-precision)"))
  (`SceneComponent.K2_SetWorldRotation` (`self.AssinationWidget`) (`KismetMathLibrary.FindLookAtRotation` (`SceneComponent.K2_GetComponentLocation` (`self.AssinationWidget`)) (`SceneComponent.K2_GetComponentLocation` (`PlayerCameraManager.TransformComponent` (`GameplayStatics.GetPlayerCameraManager` 0)))) false false)
  (`SceneComponent.K2_SetWorldRotation` (`self.HealthBar `) (`KismetMathLibrary.FindLookAtRotation` (`SceneComponent.K2_GetComponentLocation` (`self.AssinationWidget`)) (`SceneComponent.K2_GetComponentLocation` (`PlayerCameraManager.TransformComponent` (`GameplayStatics.GetPlayerCameraManager` 0)))) false false)
  (`SceneComponent.K2_SetWorldRotation` (`self.Widget`) (`KismetMathLibrary.FindLookAtRotation` (`SceneComponent.K2_GetComponentLocation` (`self.AssinationWidget`)) (`SceneComponent.K2_GetComponentLocation` (`PlayerCameraManager.TransformComponent` (`GameplayStatics.GetPlayerCameraManager` 0)))) false false))

(event `Ragdoll`
  ;[1 1 1] Ragdoll
  (`|ExecutionSequence`
    (:`then_0`
      (`KismetSystemLibrary.Delay` 2.5)
      (`PrimitiveComponent.SetSimulatePhysics` (`self.Mesh`) true))
    (:`then_1`
      (`KismetSystemLibrary.Delay` 1.2)
      (`GameplayStatics.PlaySoundAtLocation` "/Game/Audio/Attacks/SC_Death.SC_Death" (`self.K2_GetActorLocation`) (struct) 1.0 1.0 0.0 "/Game/Audio/SA_Character.SA_Character" null null null))))

(event `self.Assasination Radius.OnComponentBeginOverlap`
  (params (OverlappedComponent :type "PrimitiveComponent Object Reference") (OtherActor :type "Actor Object Reference") (OtherComp :type "PrimitiveComponent Object Reference") (OtherBodyIndex :type Integer) (bFromSweep :type Boolean) (SweepResult :type "HitResult Structure (by ref)"))
  (cast `/Game/ThirdPerson/Blueprints/BP_ThirdPersonCharacter` OtherActor)
  (`SceneComponent.SetVisibility` (`self.AssinationWidget`) true false))

(event `self.Assasination Radius.OnComponentEndOverlap`
  (params (OverlappedComponent :type "PrimitiveComponent Object Reference") (OtherActor :type "Actor Object Reference") (OtherComp :type "PrimitiveComponent Object Reference") (OtherBodyIndex :type Integer))
  (cast `/Game/ThirdPerson/Blueprints/BP_ThirdPersonCharacter` OtherActor)
  (`SceneComponent.SetVisibility` (`self.AssinationWidget`) false false))

(event `self.ReceiveAnyDamage`
  (params (Damage :type "Float (single-precision)") (DamageType :type "DamageType Object Reference") (InstigatedBy :type "Controller Object Reference") (DamageCauser :type "Actor Object Reference"))
  (`self.Stop Combo`)
  (`self.Stop Combo`)
  (`self.PlayAnimMontage` (`|GetArrayItem` (`self.HitAnims`) (`KismetMathLibrary.RandomIntegerInRange` 0 (- (`KismetArrayLibrary.Array_Length` (`self.HitAnims`)) 1))))
  (bind _asbp_third_person_character (cast `/Game/ThirdPerson/Blueprints/BP_ThirdPersonCharacter` (`GameplayStatics.GetPlayerCharacter` 0)))
  (`self.LaunchCharacter` (* (`KismetMathLibrary.GetForwardVector` (`self.K2_GetActorRotation` _asbp_third_person_character)) 700.0))
  (`GameplayStatics.PlaySoundAtLocation` "/Game/Audio/Attacks/Death2.Death2" (`self.K2_GetActorLocation`) (struct) 1.0 (`KismetMathLibrary.RandomFloatInRange` 1.5 1.3) 0.0 null null null null)
  (bind _isdead_ (`/Game/BluePrints/BPC_PlayerStats.DecreaseHealth` (`self.BPC_PlayerStats`) Damage))
  (if _isdead_
    (`PrimitiveComponent.SetCollisionObjectType` (`self.Mesh`) "ECC_PhysicsBody")
    (`PrimitiveComponent.SetSimulatePhysics` (`self.Mesh`) true)
    (`GameplayStatics.PlaySoundAtLocation` "/Game/Audio/Attacks/SC_Death.SC_Death" (`self.K2_GetActorLocation`) (struct) 1.0 1.0 0.0 "/Game/Audio/SA_Character.SA_Character" null null null)
    (`SceneComponent.SetVisibility` (`self.HealthBar `) false false)))

(event `Attack1`
  ;[0.05127 0.05127 0.05127] Combo System
  ;;[0.05127 0.05127 0.05127] Attack 1
  (`/Engine/EditorBlueprintResources/StandardMacros.DoOnce` false :!label _label
    (:`Completed`
      (`KismetSystemLibrary.Delay` 0.1)
      (`|PlayMontage` (`self.Mesh`) "/Game/Characters/RPG_Character/Animations/SwordAnimation/Attack1_Montage.Attack1_Montage"
        (:`then`
          (set `self.Attack Index` 1)
          (goto _label :!via `Reset`))))))

(event `Sword Attack Combo call from bt`
  ;[0.05127 0.05127 0.05127] Combo System
  (if (`self.CanAttack?`)
    (`self.SwordAttack`)))

(event `Attack2`
  ;[0.05127 0.05127 0.05127] Combo System
  ;;[0.05127 0.05127 0.05127] Attack 2
  ;;;[0.05127 0.05127 0.05127] Attack 1
  (`/Engine/EditorBlueprintResources/StandardMacros.DoOnce` false :!label _label_2
    (:`Completed`
      (`KismetSystemLibrary.Delay` 0.1)
      (`|PlayMontage` (`self.Mesh`) "/Game/Characters/RPG_Character/Animations/SwordAnimation/Attack2_Montage.Attack2_Montage" (`self.animspeed`)
        (:`then`
          (set `self.Attack Index` 2)
          (goto _label_2 :!via `Reset`))))))

(event `SwordAttack`
  ;[0.05127 0.05127 0.05127] Combo System
  ;;[0.05127 0.05127 0.05127] Sword Attack
  (if (`self.IsAttacking?`)
    (set `self.SaveAttack?` true)
    (else
      (set `self.IsAttacking?` true)
      (switch `int` (`self.Attack Index`) :!label _label_3
        (:`0`
          (`self.Attack1`))
        (:`1`
          (`self.Attack2`))
        (:`2`
          (`self.Attack 4`))))))

(event `Attack 3`
  ;[0.05127 0.05127 0.05127] Combo System
  ;;[0.05127 0.05127 0.05127] Attack 3
  (`/Engine/EditorBlueprintResources/StandardMacros.DoOnce` false :!label _label_4
    (:`Completed`
      (`KismetSystemLibrary.Delay` 0.1)
      (`|PlayMontage` (`self.Mesh`) "/Game/Characters/RPG_Character/Animations/SwordAnimation/Kick_Montage.Kick_Montage" (`self.animspeed`)
        (:`then`
          (set `self.Attack Index` 3)
          (goto _label_4 :!via `Reset`))))))

(event `Sword Attack Combo`
  ;[0.05127 0.05127 0.05127] Combo System
  ;;[0.05127 0.05127 0.05127] Combo
  (if (`self.SaveAttack?`)
    (set `self.SaveAttack?` false)
    (goto _label_3)
    (else
      (`self.Stop Combo`))))

(event `Attack 4`
  ;[0.05127 0.05127 0.05127] Combo System
  ;;[0.05127 0.05127 0.05127] Attack 4
  (`/Engine/EditorBlueprintResources/StandardMacros.DoOnce` false :!label _label_5
    (:`Completed`
      (`KismetSystemLibrary.Delay` 0.1)
      (`|PlayMontage` (`self.Mesh`) "/Game/Characters/RPG_Character/Animations/SwordAnimation/Attack3_Montage.Attack3_Montage" (`self.animspeed`)
        (:`then`
          (set `self.Attack Index` 4)
          (goto _label_5 :!via `Reset`))))))

(event `Stop Combo`
  ;[0.05127 0.05127 0.05127] Combo System
  ;;[0.05127 0.05127 0.05127] Stop Combo/Attack
  (set `self.IsAttacking?` false)
  (set `self.Attack Index` 0))

(event `Start Sword Trace`
  ;[0.05127 0.05127 0.05127] Sword Trace
  (bind _returnvalue (`KismetSystemLibrary.K2_SetTimerDelegate` (delegate `Sword Trace Loop`) 0.001 true))
  (set `self.SwordTraceLoop` _returnvalue))

(event `Sphere Trace`
  (bind _returnvalue (`SceneComponent.K2_GetComponentLocation` (`self.Sphere TraceAI`)))
  ;[0.05127 0.05127 0.05127] Sphere Trace (For Stab + Kick)
  (bind (_outhit _returnvalue_2) (`KismetSystemLibrary.SphereTraceSingle` :`Start` _returnvalue :`End` _returnvalue :`Radius` 25.0 :`TraceChannel` "TraceTypeQuery1" :`DrawDebugType` "ForDuration"))
  (if _returnvalue_2
    (bind (_bblockinghit _binitialoverlap _time _distance _location _impactpoint _normal _impactnormal _physmat _hitactor) (`GameplayStatics.BreakHitResult` _outhit))
    (if (`self.ActorHasTag` _hitactor "Damageable")
      (`GameplayStatics.ApplyDamage` _hitactor 10.0)
      (`GameplayStatics.PlayWorldCameraShake` "/Game/BluePrints/BP_CamShake.BP_CamShake_C" _location 0.0 2000.0)
      (`self.PlaySwordHotSound`)
      (`GameplayStatics.SpawnEmitterAtLocation` "/Game/VFX/Particles/Blood/P_Blood_Splat_Cone.P_Blood_Splat_Cone" _location (`KismetMathLibrary.MakeRotFromXY` _normal _normal) (0.4 0.4 0.4) true "AutoRelease"))))

(event `Sword Trace Loop`
  ;[0.05127 0.05127 0.05127] Sword Trace
  (bind (_outhit _returnvalue) (`KismetSystemLibrary.SphereTraceSingle` :`Start` (`SceneComponent.K2_GetComponentLocation` (`self.SwordToppoint`)) :`End` (`SceneComponent.K2_GetComponentLocation` (`self.SwordBottomPoint`)) :`Radius` 12.0 :`TraceChannel` "TraceTypeQuery1" :`DrawDebugType` "ForDuration" :`DrawTime` 0.2))
  (if _returnvalue
    (bind (_bblockinghit _binitialoverlap _time _distance _location _impactpoint _normal _impactnormal _physmat _hitactor) (`GameplayStatics.BreakHitResult` _outhit))
    (if (`self.ActorHasTag` _hitactor "Damageable")
      (`/Engine/EditorBlueprintResources/StandardMacros.DoOnce` false :!label _label_6
        (:`Completed`
          (`GameplayStatics.ApplyDamage` _hitactor 10.0)
          (`GameplayStatics.PlayWorldCameraShake` "/Game/BluePrints/BP_CamShake.BP_CamShake_C" _location 0.0 2000.0)
          (`self.PlaySwordHotSound`)
          (`GameplayStatics.SpawnEmitterAtLocation` "/Game/VFX/Particles/Blood/P_Blood_Splat_Cone.P_Blood_Splat_Cone" _location (`KismetMathLibrary.MakeRotFromXY` _normal _normal) (0.4 0.4 0.4) true "AutoRelease")
          (`KismetSystemLibrary.Delay` 0.5)
          (goto _label_6 :!via `Reset`))))))

(event `StopSwordTrace`
  ;[0.05127 0.05127 0.05127] Sword Trace
  (`KismetSystemLibrary.K2_ClearAndInvalidateTimerHandle` (`self.SwordTraceLoop`)))

(event `InvesIcon`
  (bind _widget (`self.Widget`))
  (`/Engine/EditorBlueprintResources/StandardMacros.FlipFlop`
    (:`A`
      (`SceneComponent.SetVisibility` _widget true false))
    (:`B`
      (`SceneComponent.SetVisibility` _widget false false))))

(event `PlaySwordHotSound`
  ;[0.05127 0.05127 0.05127] Sword sounds
  (`GameplayStatics.PlaySoundAtLocation` "/Game/Audio/SwordSounds/MS_SwordHit.MS_SwordHit" (`self.K2_GetActorLocation` (`self.GetOwner`)) (struct) 1.0 1.0 0.0 null null null null))

(fn `Attack`
  (returns (AnimTime :type "Float (double-precision)"))
  (`self.Sword Attack Combo call from bt`)
  (return 0.4))

(fn `StealthbBack Assassin`
  (returns (ReferenceLocation :type "Vector Structure") (AssassinRotation :type "Rotator Structure"))
  (`self.PlayAnimMontage` "/Game/Characters/RPG_Character/Animations/Assainations/Paired_Knife_Stealth_KidneyAndNeck_Vic_Montage.Paired_Knife_Stealth_KidneyAndNeck_Vic_Montage")
  (`self.Ragdoll`)
  (`SceneComponent.SetVisibility` (`self.AssinationWidget`) false false)
  (return (`SceneComponent.K2_GetComponentLocation` (`self.AssassinREf`)) (`self.K2_GetActorRotation`)))

(fn `UserConstructionScript`)