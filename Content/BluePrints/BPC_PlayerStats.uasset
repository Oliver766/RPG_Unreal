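; Stats component for the player, training dummies and AI, tracking health, stamina, XP and level.
; BeginPlay identifies the owner by cast and sets a CharacterType, which selects the health widget used at start and on damage.
; Other updates write straight to the player HUD; health and stamina decreases return true on depletion.
; Reaching MaxXP raises the level, resets XP, derives the next threshold from MaxHealth and plays two sounds.
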(event `self.ReceiveBeginPlay`
  (`KismetSystemLibrary.DelayUntilNextTick`)
  (bind _asbp_third_person_character (cast `/Game/ThirdPerson/Blueprints/BP_ThirdPersonCharacter` (`self.GetOwner`))
    (:`then`
      (set `self.Play charachter` _asbp_third_person_character)
      (set `self.Is Player` true)
      (`ProgressBar.SetPercent` (`/Game/UI/WB_HUD.StamiaBar` (`/Game/ThirdPerson/Blueprints/BP_ThirdPersonCharacter.HUD Widget` (`self.Play charachter`))) (/ (`self.CurrentStamia`) (`self.MaxStamia`)))
      (set `self.Character Type` "NewEnumerator0"))
    (:`CastFailed`
      (bind _asbp_dummy (cast `/Game/BluePrints/BP_Dummy` (`self.GetOwner`))
        (:`then`
          (set `self.As BP Dummy` _asbp_dummy)
          (set `self.Is Player` false)
          (set `self.Character Type` "NewEnumerator1"))
        (:`CastFailed`
          (bind _asbp_ai (cast `/Game/AI/BP_AI` (`self.GetOwner`)))
          (set `self. BP AI` _asbp_ai)
          (set `self.Character Type` "NewEnumerator2")))))
  (`ProgressBar.SetPercent` (select `/Game/BluePrints/E_CharacterTypes` (`self.Character Type`) :`NewEnumerator0` (`/Game/UI/WB_HUD.HealthBar` (`/Game/ThirdPerson/Blueprints/BP_ThirdPersonCharacter.HUD Widget` (`self.Play charachter`))) :`NewEnumerator1` (`/Game/UI/DummyHealthbar.HealthBar` (`/Game/BluePrints/BP_Dummy.DummyHealthbar` (`self.As BP Dummy`))) :`NewEnumerator2` (`/Game/UI/DummyHealthbar.HealthBar` (`/Game/AI/BP_AI.Healthbar UI` (`self. BP AI`)))) (/ (`self.CurrentHealth`) (`self.MaxHealth`)))
  (`TextBlock.SetText` (select `/Game/BluePrints/E_CharacterTypes` (`self.Character Type`) :`NewEnumerator0` (`/Game/UI/WB_HUD.HealthText` (`/Game/ThirdPerson/Blueprints/BP_ThirdPersonCharacter.HUD Widget` (`self.Play charachter`))) :`NewEnumerator1` (`/Game/UI/DummyHealthbar.HealthText` (`/Game/BluePrints/BP_Dummy.DummyHealthbar` (`self.As BP Dummy`))) :`NewEnumerator2` (`/Game/UI/DummyHealthbar.HealthText` (`/Game/AI/BP_AI.Healthbar UI` (`self. BP AI`)))) (`KismetTextLibrary.Conv_DoubleToText` (`self.CurrentHealth`) "HalfToEven"))
  (if (`self.Is Player`)
    (`ProgressBar.SetPercent` (`/Game/UI/WB_HUD.LevelBar` (`/Game/ThirdPerson/Blueprints/BP_ThirdPersonCharacter.HUD Widget` (`self.Play charachter`))) (/ (`self.XP`) (`self.MaxXP`)))
    (`TextBlock.SetText` (`/Game/UI/WB_HUD.XP` (`/Game/ThirdPerson/Blueprints/BP_ThirdPersonCharacter.HUD Widget` (`self.Play charachter`))) (`|FormatText` "{Current XP} / {Max XP}" (`self.XP`) (`self.MaxXP`)))
    (`TextBlock.SetText` (`/Game/UI/WB_HUD.Leveltxt` (`/Game/ThirdPerson/Blueprints/BP_ThirdPersonCharacter.HUD Widget` (`self.Play charachter`))) (`KismetTextLibrary.Conv_IntToText` (`self.Level`)))))

(fn `DecreaseHealth`
  (params (Damage :type "Float (double-precision)"))
  (returns (`IsDead?` :type Boolean))
  ;[1 1 1] Decrease Health
  (if (not (<= (`self.CurrentHealth`) 0.0))
    (bind _output_get (set `self.CurrentHealth` (- (`self.CurrentHealth`) Damage)))
    (`ProgressBar.SetPercent` (select `/Game/BluePrints/E_CharacterTypes` (`self.Character Type`) :`NewEnumerator0` (`/Game/UI/WB_HUD.HealthBar` (`/Game/ThirdPerson/Blueprints/BP_ThirdPersonCharacter.HUD Widget` (`self.Play charachter`))) :`NewEnumerator1` (`/Game/UI/DummyHealthbar.HealthBar` (`/Game/BluePrints/BP_Dummy.DummyHealthbar` (`self.As BP Dummy`))) :`NewEnumerator2` (`/Game/UI/DummyHealthbar.HealthBar` (`/Game/AI/BP_AI.Healthbar UI` (`self. BP AI`)))) (/ _output_get (`self.MaxHealth`)))
    (`TextBlock.SetText` (select `/Game/BluePrints/E_CharacterTypes` (`self.Character Type`) :`NewEnumerator0` (`/Game/UI/WB_HUD.HealthText` (`/Game/ThirdPerson/Blueprints/BP_ThirdPersonCharacter.HUD Widget` (`self.Play charachter`))) :`NewEnumerator1` (`/Game/UI/DummyHealthbar.HealthText` (`/Game/BluePrints/BP_Dummy.DummyHealthbar` (`self.As BP Dummy`))) :`NewEnumerator2` (`/Game/UI/DummyHealthbar.HealthText` (`/Game/AI/BP_AI.Healthbar UI` (`self. BP AI`)))) (`KismetTextLibrary.Conv_DoubleToText` (`self.CurrentHealth`) "HalfToEven"))
    (if (<= (`self.CurrentHealth`) 0.0)
      _
      (else
        (return false))))
  (return true))

(fn `DecreaseStamia`
  (params (Depletion :type "Float (double-precision)"))
  (returns (`No Stamia Left` :type Boolean))
  (if (not (<= (`self.CurrentStamia`) 0.0))
    (set `self.CurrentStamia` (- (`self.CurrentStamia`) Depletion))
    (`ProgressBar.SetPercent` (`/Game/UI/WB_HUD.StamiaBar` (`/Game/ThirdPerson/Blueprints/BP_ThirdPersonCharacter.HUD Widget` (`self.Play charachter`))) (/ (`self.CurrentStamia`) (`self.MaxStamia`)))
    (if (<= (`self.CurrentStamia`) 0.0)
      _
      (else
        (return false))))
  (return true))

(fn `Increas max Stamia`
  (params (IncreasStamia :type "Float (double-precision)"))
  (set `self.MaxStamia` (+ (`self.MaxStamia`) IncreasStamia))
  (`ProgressBar.SetPercent` (`/Game/UI/WB_HUD.StamiaBar` (`/Game/ThirdPerson/Blueprints/BP_ThirdPersonCharacter.HUD Widget` (`self.Play charachter`))) (/ (`self.CurrentStamia`) (`self.MaxStamia`))))

(fn `Increase Level`
  (params (`Added Level` :type Integer))
  (set `self.Level` (+ (`self.Level`) `Added Level`))
  (set `self.MaxXP` (+ (`self.MaxHealth`) 150.0))
  (set `self.XP` 0.0)
  (`TextBlock.SetText` (`/Game/UI/WB_HUD.Leveltxt` (`/Game/ThirdPerson/Blueprints/BP_ThirdPersonCharacter.HUD Widget` (`self.Play charachter`))) (`KismetTextLibrary.Conv_IntToText` (`self.Level`)))
  (`GameplayStatics.PlaySound2D` "/Game/Audio/UI/Levelup1.Levelup1" 1.0 1.0 0.0 null null)
  (`GameplayStatics.PlaySound2D` "/Game/Audio/UI/LevelUp2.LevelUp2" 1.0 1.0 0.0 null null))

(fn `Increase MaxHealth`
  (params (Regen :type "Float (double-precision)"))
  (bind _hud_widget (`/Game/ThirdPerson/Blueprints/BP_ThirdPersonCharacter.HUD Widget` (`self.Play charachter`)))
  (set `self.MaxHealth` (+ (`self.MaxHealth`) Regen))
  (`ProgressBar.SetPercent` (`/Game/UI/WB_HUD.HealthBar` _hud_widget) (/ (`self.CurrentHealth`) (`self.MaxHealth`)))
  (`TextBlock.SetText` (`/Game/UI/WB_HUD.HealthText` _hud_widget) (`KismetTextLibrary.Conv_DoubleToText` (`self.CurrentHealth`) "HalfToEven")))

(fn `Increase XP`
  (params (`Added XP` :type "Float (double-precision)"))
  (set `self.XP` (+ (`self.XP`) `Added XP`))
  (if (>= (`self.XP`) (`self.MaxXP`))
    (`self.Increase Level` 1))
  (`ProgressBar.SetPercent` (`/Game/UI/WB_HUD.LevelBar` (`/Game/ThirdPerson/Blueprints/BP_ThirdPersonCharacter.HUD Widget` (`self.Play charachter`))) (/ (`self.XP`) (`self.MaxXP`)))
  (`TextBlock.SetText` (`/Game/UI/WB_HUD.XP` (`/Game/ThirdPerson/Blueprints/BP_ThirdPersonCharacter.HUD Widget` (`self.Play charachter`))) (`|FormatText` "{Current XP} / {Max XP}" (`self.XP`) (`self.MaxXP`))))

(fn `IncreaseHealth`
  (params (`Add Health` :type "Float (double-precision)"))
  (bind _hud_widget (`/Game/ThirdPerson/Blueprints/BP_ThirdPersonCharacter.HUD Widget` (`self.Play charachter`)))
  ;[0.05127 0.05127 0.05127] Increase Health
  (set `self.CurrentHealth` (+ (`self.CurrentHealth`) `Add Health`))
  (if (> (`self.CurrentHealth`) (`self.MaxHealth`))
    (set `self.CurrentHealth` (`self.MaxHealth`)))
  (`ProgressBar.SetPercent` (`/Game/UI/WB_HUD.HealthBar` _hud_widget) (/ (`self.CurrentHealth`) (`self.MaxHealth`)))
  (`TextBlock.SetText` (`/Game/UI/WB_HUD.HealthText` _hud_widget) (`KismetTextLibrary.Conv_DoubleToText` (`self.CurrentHealth`) "HalfToEven")))

(fn `IncreaseStamia`
  (params (Increase :type "Float (double-precision)"))
  (set `self.CurrentStamia` (+ (`self.CurrentStamia`) Increase))
  (if (> (`self.CurrentStamia`) (`self.MaxStamia`))
    (set `self.CurrentStamia` (`self.MaxStamia`)))
  (`ProgressBar.SetPercent` (`/Game/UI/WB_HUD.StamiaBar` (`/Game/ThirdPerson/Blueprints/BP_ThirdPersonCharacter.HUD Widget` (`self.Play charachter`))) (/ (`self.CurrentStamia`) (`self.MaxStamia`))))